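; Turtlebot3 Waffle robot Blueprint that provides an orbit camera on a spring arm.
; On BeginPlay it sets the spring arm length from the CameraArmLength variable.
; LookRight yaws the arm, while LookUp applies inverted pitch and then clamps it to keep the view from flipping over the top or bottom.
; The graphs contain only this camera logic, with no movement or per-frame behavior.
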(event `self.ReceiveBeginPlay`
  (set `SpringArmComponent.TargetArmLength` (`self.CameraArmLength`) (`self.SpringArm`)))

(event `InputAxis|LookUp`
  (params (AxisValue :type "Float (single-precision)"))
  (bind _springarm (`self.SpringArm`))
  (bind (_relativerotation_roll _relativerotation_pitch _relativerotation_yaw) (`KismetMathLibrary.BreakRotator` (`SceneComponent.RelativeRotation` _springarm)))
  ;[1 1 1] Look
  (`SceneComponent.K2_AddRelativeRotation` _springarm (`KismetMathLibrary.MakeRotator` 0.0 (* AxisValue -1.0)) false false)
  (`SceneComponent.K2_SetRelativeRotation` _springarm (`KismetMathLibrary.MakeRotator` _relativerotation_roll (`KismetMathLibrary.FClamp` _relativerotation_pitch -75.0 75.0) _relativerotation_yaw) false false))

(event `InputAxis|LookRight`
  (params (AxisValue :type "Float (single-precision)"))
  ;[1 1 1] Look
  (`SceneComponent.K2_AddRelativeRotation` (`self.SpringArm`) (`KismetMathLibrary.MakeRotator` 0.0 0.0 AxisValue) false false))

(fn `UserConstructionScript`)